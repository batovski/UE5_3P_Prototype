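; Character component that gives its owner wall climbing and vaulting, plus stamina-limited sprinting.
; VaultJump line-traces wall face, height and thickness to pick climb or vault, then disables capsule collision, sets Flying and plays montages on player character 0.
; A montage-length timer ends vaults, while climbs restore collision and walking immediately.
; A parkour state gates actions and drives UpdateStamina's sprint drain or delayed regeneration; parkour attempts also cost stamina.
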(event EventBeginPlay
  (bind _returnvalue (Components|GetOwner))
  (Variables|Default|SetActor _returnvalue)
  (Variables|Default|SetCharacterMovement (Actor|GetComponentbyClass _returnvalue "/Script/Engine.CharacterMovementComponent"))
  (Variables|Default|SetCapsuleComponent (Actor|GetComponentbyClass _returnvalue "/Script/Engine.CapsuleComponent")))

(event EventTick
  (params (DeltaSeconds :type Float%20%28single-precision%29)))

(fn Vault/Jump
  (bind _returnvalue (Game|GetPlayerCharacter 0))
  (bind _returnvalue_2 (Game|GetPlayerCharacter 0))
  (bind _wallmaxheight (Variables|Default|GetWallMaxHeight))
  (bind _actor (Variables|Default|GetActor))
  (bind _actor_2 (Variables|Default|GetActor))
  (bind _actor_3 (Variables|Default|GetActor))
  (bind _actor_4 (Variables|Default|GetActor))
  (bind _actor_5 (Variables|Default|GetActor))
  (bind _actor_6 (Variables|Default|GetActor))
  (bind _returnvalue_3 (Transformation|GetActorLocation _actor))
  (bind _returnvalue_4 (Transformation|GetActorRotation _actor_3))
  (bind _returnvalue_5 (Transformation|GetActorLocation _actor_6))
  (bind _returnvalue_6 (Transformation|GetActorLocation _actor_2))
  (bind _returnvalue_7 (Transformation|GetActorLocation _actor_4))
  (bind _returnvalue_8 (Transformation|GetActorLocation _actor_5))
  (bind _returnvalue_9 (- _returnvalue_3 "0.000000,0.000000,44.000000"))
  (bind _returnvalue_10 (+ _returnvalue_7 (Math|Vector|MakeVector 0.0 0.0 _wallmaxheight)))
  (LocalVariables|SetCanClimb? true)
  (Utilities|FlowControl|Sequence
    (:then_0
      (if (not (LocalVariables|GetIsClimbing?))
        ;[1 1 1] Detact the Wall
        (bind (_outhit _returnvalue_11) (Collision|LineTraceForObjects _returnvalue_9 (+ _returnvalue_9 (* (Transformation|GetActorForwardVector (Variables|Default|GetActor)) (Math|Vector|MakeVector 7e+01 7e+01 7e+01))) (Utilities|Array|MakeArray "ObjectTypeQuery1") false 0 "ForDuration"))
        (if _returnvalue_11
          (LocalVariables|SetWall%20Location (.Location (Collision|BreakHitResult _outhit)))
          (LocalVariables|SetWall%20Normal (.Normal (Collision|BreakHitResult _outhit)))
          ;[1 1 1] Detact the height of the wall
          (bind (_outhit_2 _returnvalue_12) (Collision|LineTraceForObjects (+ (+ (LocalVariables|GetWall%20Location) (* (Math|Vector|GetForwardVector (Math|Rotator|MakeRotfromX (LocalVariables|GetWall%20Normal))) (Math|Vector|MakeVector -1e+01 -1e+01 -1e+01))) (Math|Vector|MakeVector 0.0 0.0 (Variables|Default|GetWallMaxHeight))) (+ (LocalVariables|GetWall%20Location) (* (Math|Vector|GetForwardVector (Math|Rotator|MakeRotfromX (LocalVariables|GetWall%20Normal))) (Math|Vector|MakeVector -1e+01 -1e+01 -1e+01))) (Utilities|Array|MakeArray "ObjectTypeQuery1") false 0 "ForDuration"))
          (if _returnvalue_12
            (LocalVariables|SetWall%20Height (.Location (Collision|BreakHitResult _outhit_2)))
            (Utilities|FlowControl|Sequence
              (:then_0
                (if (> (.z (- (LocalVariables|GetWall%20Height) (LocalVariables|GetWall%20Location))) 6e+01)
                  (LocalVariables|SetShouldPlayerClimb? true)
                  (else
                    (LocalVariables|SetShouldPlayerClimb? false))))
              (:then_1
                (bind (_outhit_3 _returnvalue_13) (Collision|LineTraceForObjects (+ (+ (LocalVariables|GetWall%20Location) (* (Math|Vector|GetForwardVector (Math|Rotator|MakeRotfromX (LocalVariables|GetWall%20Normal))) (Math|Vector|MakeVector -5e+01 -5e+01 -5e+01))) (Math|Vector|MakeVector 0.0 0.0 (Variables|Default|GetWallMaxHeight))) (- (+ (+ (LocalVariables|GetWall%20Location) (* (Math|Vector|GetForwardVector (Math|Rotator|MakeRotfromX (LocalVariables|GetWall%20Normal))) (Math|Vector|MakeVector -5e+01 -5e+01 -5e+01))) (Math|Vector|MakeVector 0.0 0.0 (Variables|Default|GetWallMaxHeight))) "0.000000,0.000000,350.000000") (Utilities|Array|MakeArray "ObjectTypeQuery1") false 0 "ForDuration"))
                (if _returnvalue_13
                  (LocalVariables|SetWallHeight2 (.Location (Collision|BreakHitResult _outhit_3)))
                  (Utilities|FlowControl|Sequence
                    (:then_0
                      (if (> (.z (- (LocalVariables|GetWall%20Height) (LocalVariables|GetWallHeight2))) 3e+01)
                        (LocalVariables|SetIsWallThick? false)
                        (else
                          (LocalVariables|SetIsWallThick? true))))
                    (:then_1
                      (if (LocalVariables|GetShouldPlayerClimb?) :!label _label
                        (if (Pawn|Components|CharacterMovement|IsWalking (Variables|Default|GetCharacterMovement))
                          ;[1 1 1] ClimbUp
                          ;;[1 1 1] Check if there is something above
                          (Utilities|FlowControl|Sequence
                            (:then_0
                              (bind _returnvalue_14 (Collision|LineTraceForObjects _returnvalue_10 (+ _returnvalue_10 (* (Transformation|GetActorForwardVector (Variables|Default|GetActor)) "70.000000,70.000000,70.000000")) (Utilities|Array|MakeArray "ObjectTypeQuery1") false 0 "ForDuration"))
                              (if _returnvalue_14
                                (LocalVariables|SetCanClimb? false))
                              (Collision|LineTraceForObjects _returnvalue_8 (+ _returnvalue_8 (Math|Vector|MakeVector 0.0 0.0 (Variables|Default|GetWallMaxHeight))) (Utilities|Array|MakeArray "ObjectTypeQuery1") false 0 "ForDuration"))
                            (:then_1
                              (if (LocalVariables|GetCanClimb?)
                                (LocalVariables|SetIsClimbing? true)
                                (Transformation|SetActorRotation (Variables|Default|GetActor) (Math|Rotator|MakeRotfromX (* (LocalVariables|GetWall%20Normal) "-1.000000,-1.000000,-1.000000")))
                                (Collision|SetCollisionEnabled (Variables|Default|GetCapsuleComponent) "NoCollision")
                                (Pawn|Components|CharacterMovement|SetMovementMode (Variables|Default|GetCharacterMovement) "MOVE_Flying" 0)
                                (Transformation|SetActorRotation (Variables|Default|GetActor) (Math|Rotator|MakeRotator (.roll _returnvalue_4) (.pitch _returnvalue_4) (+ (.yaw (Math|Rotator|MakeRotfromX (LocalVariables|GetWall%20Normal))) 1.8e+02)))
                                (Transformation|SetActorLocation (Variables|Default|GetActor) (Math|Vector|MakeVector (.x _returnvalue_5) (.y _returnvalue_5) (- (.z (LocalVariables|GetWall%20Height)) 44.0)) false false)
                                (Animation|PlayAnimMontage _returnvalue_2 "/Game/Characters/Parkour/MQ_Climb_RM_Montage.MQ_Climb_RM_Montage" 1.0 "None")
                                (if (LocalVariables|GetIsWallThick?)
                                  (Collision|SetCollisionEnabled (Variables|Default|GetCapsuleComponent) "QueryAndPhysics")
                                  (Pawn|Components|CharacterMovement|SetMovementMode (Variables|Default|GetCharacterMovement) "MOVE_Walking" 0)
                                  (else
                                    (Transformation|SetActorLocation (Variables|Default|GetActor) (+ (Transformation|GetActorLocation (Variables|Default|GetActor)) (* (LocalVariables|GetWall%20Normal) "15.000000,15.000000,15.000000")) true false)
                                    (Animation|PlayAnimMontage _returnvalue_2 "/Game/Characters/Parkour/MQ_JumpingDownFromWall_RM_Montage.MQ_JumpingDownFromWall_RM_Montage" 1.0 "None")
                                    (Collision|SetCollisionEnabled (Variables|Default|GetCapsuleComponent) "QueryAndPhysics")
                                    (Pawn|Components|CharacterMovement|SetMovementMode (Variables|Default|GetCharacterMovement) "MOVE_Walking" 0)))
                                (LocalVariables|SetIsClimbing? false)
                                (else
                                  (LocalVariables|SetIsExecuted? false)))))
                          (else
                            (LocalVariables|SetIsExecuted? false)))
                        (else
                          ;[1 1 1] Vaulting
                          (LocalVariables|SetIsClimbing? true)
                          (Transformation|SetActorRotation (Variables|Default|GetActor) (Math|Rotator|MakeRotfromX (* (LocalVariables|GetWall%20Normal) "-1.000000,-1.000000,-1.000000")) true)
                          (Collision|SetCollisionEnabled (Variables|Default|GetCapsuleComponent) "NoCollision")
                          (Pawn|Components|CharacterMovement|SetMovementMode (Variables|Default|GetCharacterMovement) "MOVE_Flying" 0)
                          (if (LocalVariables|GetIsWallThick?)
                            (Transformation|SetActorLocation (Variables|Default|GetActor) (+ (Transformation|GetActorLocation (Variables|Default|GetActor)) (* (Math|Vector|GetForwardVector (Math|Rotator|MakeRotfromX (LocalVariables|GetWall%20Normal))) "40.000000,40.000000,40.000000")) true false)
                            (Variables|Default|SetParkourState "NewEnumerator1")
                            (bind _returnvalue_15 (Animation|PlayAnimMontage _returnvalue 0 1.0 "None"))
                            (Utilities|Time|SetTimerbyFunctionName 0 "VaultCloseGate" _returnvalue_15)
                            (else
                              (Transformation|SetActorLocation (Variables|Default|GetActor) (+ (Transformation|GetActorLocation (Variables|Default|GetActor)) (* (Math|Vector|GetForwardVector (Math|Rotator|MakeRotfromX (LocalVariables|GetWall%20Normal))) "40.000000,40.000000,40.000000")) true false)
                              (Transformation|SetActorLocation (Variables|Default|GetActor) (Math|Vector|MakeVector (.x _returnvalue_6) (.y _returnvalue_6) (+ (.z _returnvalue_6) 11.5)) true false)
                              (Variables|Default|SetParkourState "NewEnumerator0")
                              (bind _returnvalue_16 (Animation|PlayAnimMontage _returnvalue 0 1.0 "None"))
                              (Utilities|Time|SetTimerbyFunctionName 0 "VaultCloseGate" _returnvalue_16)))))))
                  (else
                    (LocalVariables|SetIsWallThick? false)
                    (goto _label)))))
            (else
              (LocalVariables|SetIsExecuted? false)))
          (else
            (LocalVariables|SetIsExecuted? false)))))
    (:then_1
      (return (LocalVariables|GetIsExecuted?)))))

(fn VaultCloseGate
  (Collision|SetCollisionEnabled (Variables|Default|GetCapsuleComponent) "QueryAndPhysics")
  (Pawn|Components|CharacterMovement|SetMovementMode (Variables|Default|GetCharacterMovement) "MOVE_Walking" 0)
  (Variables|Default|SetParkourState "NewEnumerator2"))

(fn CheckState
  (params (State :type E_ParkourEnumType%20Enum :default "NewEnumerator2"))
  (return (Utilities|Enum|Equal(Enum) State (Variables|Default|GetParkourState))))

(fn DecreaseStamina
  (params (Value :type Float%20%28double-precision%29))
  (Variables|Stamina|SetStamina (Math|Float|Clamp(Float) (- (Variables|Stamina|GetStamina) Value) 0.0 (Variables|Stamina|GetMaxStamina)))
  (Variables|Stamina|SetCurrentStaminaRegenDelay (Variables|Stamina|GetStamina%20Regen%20Delay)))

(fn StartSprint
  (bind _charactermovement (Variables|Default|GetCharacterMovement))
  (if (> (Math|Vector|VectorLength (Variables|/Script/Engine.MovementComponent|GetVelocity _charactermovement)) 3.0)
    (Variables|/Script/Engine.CharacterMovementComponent|SetMaxWalkSpeed _charactermovement (Variables|Stamina|GetSprint%20Max%20Speed))
    (Variables|Default|SetParkourState "NewEnumerator3")))

(fn StopSprint
  (Variables|/Script/Engine.CharacterMovementComponent|SetMaxWalkSpeed (Variables|Default|GetCharacterMovement) (Variables|Stamina|GetWalkSpeed))
  (Variables|Default|SetParkourState "NewEnumerator2")
  (Variables|Stamina|SetCurrentStaminaRegenDelay (/ (Variables|Stamina|GetStamina%20Regen%20Delay) 2.0)))

(fn UpdateStamina
  (params (Time :type Float%20%28double-precision%29))
  (bind _match_ (CallFunction|CheckState "NewEnumerator3"))
  (if _match_
    ;[1 1 1] Drain Stamina
    (bind _output_get (Variables|Stamina|SetStamina (Math|Float|Clamp(Float) (- (Variables|Stamina|GetStamina) (Variables|Stamina|GetSprintStaminaCost)) 0.0 (Variables|Stamina|GetMaxStamina))))
    (if (== _output_get 0.0)
      (CallFunction|StopSprint))
    (else
      ;[1 1 1] Regen Stamina
      (if (<= (Variables|Stamina|GetCurrentStaminaRegenDelay) 0.0)
        (Variables|Stamina|SetStamina (Math|Float|Clamp(Float) (+ (Variables|Stamina|GetStamina) (Variables|Stamina|GetStaminaRecoveryCost)) 0.0 (Variables|Stamina|GetMaxStamina)))
        (else
          (Variables|Stamina|SetCurrentStaminaRegenDelay (Math|Float|Clamp(Float) (- (Variables|Stamina|GetCurrentStaminaRegenDelay) Time) 0.0 (Variables|Stamina|GetStamina%20Regen%20Delay))))))))

(fn ParkourAction
  (bind _match_ (CallFunction|CheckState "NewEnumerator2"))
  (bind _match__2 (CallFunction|CheckState "NewEnumerator3"))
  (if (or _match_ _match__2)
    (CallFunction|DecreaseStamina (Variables|Stamina|GetJumpStaminaCost))
    (bind _exsecuted_ (CallFunction|Vault/Jump))
    (if _exsecuted_
      (return true)
      (else
        (return false)))))